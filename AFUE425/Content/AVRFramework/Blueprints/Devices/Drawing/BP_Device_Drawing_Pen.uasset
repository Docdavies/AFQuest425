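; Grabbable VR pen device that draws spline strokes in the world, with adjustable colour and thumbstick-controlled tip size.
; Holding trigger spawns a BP_Stroke that Tick extends from the Arrow's transform, with size-scaled haptics.
; On trigger or pen release, the preview stroke is destroyed and its points go to a server event that rebuilds it for all clients.
; A face button toggles a camera-facing colour palette, removed with the pen's release or deletion.
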(event `EndDrawing`
  ;[1 1 1] On Triggerpressed create SplineDrawing Actor
  (set `self.IsDrawing` false)
  (bind _stroke (`self.Stroke`)
    (:`then`
      (`self.Server_SpawnStrokeOnAllClients` (`/Game/AVRFramework/Blueprints/Devices/Drawing/BP_Stroke.AnnotationPointTransforms` _stroke) (`self.SplineMaterial`))
      (`self.K2_DestroyActor` (`self.Stroke`)))
    (:`else`)))

(event `Server_SpawnStrokeOnAllClients`
  (params (TransformSplinePoints :type "Array of Transform Structure") (MaterialToUse :type "MaterialInterface Object Reference"))
  (bind _returnvalue (`|SpawnActorFromClass` "/Game/AVRFramework/Blueprints/Devices/Drawing/BP_Stroke.BP_Stroke_C" (`KismetMathLibrary.MakeTransform` (.location (`|GetArrayItem` TransformSplinePoints))) "AlwaysSpawn" "OverrideRootScale" null (0.0 0.0 0.0) (0.0 0.0 0.0) (struct) 1.0 MaterialToUse null))
  (`/Game/AVRFramework/Blueprints/Devices/Drawing/BP_Stroke.BuildStrokeFromTransformArray` _returnvalue TransformSplinePoints MaterialToUse))

(event `self.Comp_Grab.KeyInput`
  (params (Key :type "/Game/AVRFramework/Enums/Enum_Controller_Buttons Enum" :default "NewEnumerator1") (Set :type Boolean))
  (bind _arrow (`self.Arrow`))
  (bind _returnvalue (+ (`self.K2_GetActorLocation`) (0.0 0.0 20.0)))
  ;[1 1 1] On Triggerpressed create SplineDrawing Actor
  (switch `/Game/AVRFramework/Enums/Enum_Controller_Buttons` Key
    (:`NewEnumerator0`
      (if Set
        (bind _returnvalue_2 (`|SpawnActorFromClass` "/Game/AVRFramework/Blueprints/Devices/Drawing/BP_Stroke.BP_Stroke_C" (`KismetMathLibrary.MakeTransform` (`SceneComponent.K2_GetComponentLocation` (`self.Arrow`))) "Undefined" "OverrideRootScale" null (`SceneComponent.K2_GetComponentLocation` _arrow) (`SceneComponent.GetForwardVector` _arrow) (`SceneComponent.K2_GetComponentRotation` _arrow) 1.0 (`self.SplineMaterial`) null))
        (set `self.Stroke` _returnvalue_2)
        (set `self.IsDrawing` true)
        (else
          (`self.EndDrawing`))))
    (:`NewEnumerator4`
      (if Set
        (`/Engine/EditorBlueprintResources/StandardMacros.IsValid` (`self.ColorPallet`)
          (:`Is Valid`
            (`/Game/AVRFramework/Libraries/FLib_Utility.DeleteActor` (`self.ColorPallet`) "NewEnumerator1")
            (set `self.ColorPallet` null))
          (:`Is Not Valid`
            (bind _grabbingpawn (`/Game/AVRFramework/Blueprints/Components/Interaction/Comp_Grab.CurrentlyGrabbedBy` (`self.Comp_Grab`)))
            (bind _returnvalue_3 (`|SpawnActorFromClass` "/Game/AVRFramework/Blueprints/UI/Utils/BP_ColorPallet.BP_ColorPallet_C" (`KismetMathLibrary.MakeTransform` _returnvalue (`KismetMathLibrary.FindLookAtRotation` _returnvalue (`SceneComponent.K2_GetComponentLocation` (`/Game/AVRFramework/Blueprints/Pawn/BP_Pawn_Base.GetCameraComponent` _grabbingpawn)))) "Undefined" "OverrideRootScale" null self null))
            (set `self.ColorPallet` _returnvalue_3)))))))

(event `ChangeDrawingMaterial`
  (params (SplineMaterial :type "MaterialInterface Object Reference"))
  ;[1 1 1] Handle Change Drawing Color
  (bind _output_get (set `self.SplineMaterial` SplineMaterial))
  (bind _returnvalue (`KismetMaterialLibrary.CreateDynamicMaterialInstance` _output_get _output_get))
  (bind _output_get_2 (set `self.DynamicSplineMaterial` _returnvalue))
  (bind _returnvalue_2 (`MaterialInstanceDynamic.K2_GetVectorParameterValue` _output_get_2 "Color"))
  (bind _returnvalue_3 (`KismetMathLibrary.Conv_LinearColorToVector` _returnvalue_2))
  (`MeshComponent.SetVectorParameterValueOnMaterials` (`self.PenMesh`) "Color" _returnvalue_3)
  (`MeshComponent.SetVectorParameterValueOnMaterials` (`self.Tip`) "Color" (/ _returnvalue_3 3.0)))

(event `self.Comp_Grab.Thumbstick`
  (params (UpAxis :type "Float (single-precision)") (RightAxis :type "Float (single-precision)"))
  (bind _relativescale3d_x (`KismetMathLibrary.BreakVector` (`SceneComponent.RelativeScale3D` (`self.Tip`))))
  ;[1 1 1] Change Drawing Size based on Thumbstick
  (bind _output_get (set `self.CurrentScale` (`KismetMathLibrary.FClamp` (+ (`self.CurrentScale`) (* RightAxis 0.2)) (`self.MinScale`) (`self.MaxScale`))))
  (`SceneComponent.SetRelativeScale3D` (`self.Tip`) (`KismetMathLibrary.MakeVector` _relativescale3d_x _output_get _output_get)))

(event `self.ReceiveTick`
  (params (DeltaSeconds :type "Float (single-precision)"))
  (bind _arrow (`self.Arrow`))
  ;[1 1 1] Event Tick
  (`parent.ReceiveTick` DeltaSeconds)
  (set `self.DeltaSeconds` DeltaSeconds)
  ;[1 1 1] Create New Drawing Spline Points
  (if (`self.IsDrawing`)
    (`/Game/AVRFramework/Blueprints/Devices/Drawing/BP_Stroke.UpdateStroke` (`self.Stroke`) (`SceneComponent.K2_GetComponentRotation` _arrow) (`SceneComponent.K2_GetComponentLocation` _arrow) (`SceneComponent.GetForwardVector` _arrow) (`self.CurrentScale`))
    (`/Game/AVRFramework/Libraries/Lib_Core.SetHaptics` (`/Game/AVRFramework/Blueprints/Components/Interaction/Comp_Grab.GrabbingMotionController` (`self.Comp_Grab`)) "NewEnumerator1" "NewEnumerator4" 0.0 (`KismetMathLibrary.MapRangeUnclamped` (`self.CurrentScale`) 0.1 1.0 0.1 0.3))))

(event `self.Comp_Grab.ActorReleased`
  (params (ReleasingPawn :type "/Game/AVRFramework/Blueprints/Pawn/BP_Pawn_Base Object Reference") (ReleasingActor :type "Actor Object Reference") (ReleasingMotionController :type "/Game/AVRFramework/Blueprints/VR/MotionControllers/BP_MotionController Object Reference") (ReleasingMComp :type "/Game/AVRFramework/Blueprints/VR/MotionComponents/BP_MComp Object Reference"))
  ;[1 1 1] Destroy Color Pallet if valid
  (`self.EndDrawing`)
  (bind _colorpallet (`self.ColorPallet`)
    (:`then`
      (`/Game/AVRFramework/Libraries/FLib_Utility.DeleteActor` _colorpallet "NewEnumerator1"))
    (:`else`)))

(event `self.Comp_Delete.BeforeDelete`
  ;[1 1 1] Delete Color Pallet if Pen is destroyed
  (`/Game/AVRFramework/Libraries/FLib_Utility.DeleteActor` (`self.ColorPallet`) "NewEnumerator1"))

(fn `UserConstructionScript`
  (`parent.UserConstructionScript`)
  (`self.ChangeDrawingMaterial` (`self.SplineMaterial`)))