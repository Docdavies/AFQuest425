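; BP_Photo is a photo actor for the AVRFramework camera device that displays a picture on its static mesh.
; MakePhoto receives a HelperPhoto, stores it if valid, and creates a dynamic material instance on the mesh's first material slot.
; It then feeds the helper's TextureTarget into that material's Texture parameter; the actor has no other active logic.
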(event `MakePhoto`
  (params (HelperPhoto :type "/Game/AVRFramework/Blueprints/Helpers/BP_Helper_Photo Object Reference"))
  ;[1 1 1] Fill Texture from Picture Index
  (`/Engine/EditorBlueprintResources/StandardMacros.IsValid` HelperPhoto
    (:`Is Valid`
      (bind _output_get (set `self.HelperPhoto` HelperPhoto))
      (bind _returnvalue (`PrimitiveComponent.CreateDynamicMaterialInstance` (`self.StaticMesh_0`) 0 null "None"))
      (`MaterialInstanceDynamic.SetTextureParameterValue` _returnvalue "Texture" (`/Game/AVRFramework/Blueprints/Helpers/BP_Helper_Photo.TextureTarget` _output_get)))))

(fn `UserConstructionScript`
  (`parent.UserConstructionScript`))