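; Grabbable VR camera device with a live viewfinder, selfie mode and gallery mode.
; While held outside gallery mode, a low-res scene capture refreshes each tick, and the trigger shoots a high-res capture into a spawned BP_Helper_Photo's render target, with sound and haptics.
; Face buttons toggle selfie mode, which animates the capture handle around, and gallery mode, which shows a widget whose Spawn Photo command creates a BP_Photo from a helper.
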(event `self.ReceiveBeginPlay`
  ;[1 1 1] Initialize
  (`parent.ReceiveBeginPlay`)
  (`self.SetGalleryMode` (`self.GalleryMode`)))

(event `self.ReceiveTick`
  (params (DeltaSeconds :type "Float (single-precision)"))
  (`parent.ReceiveTick` DeltaSeconds)
  ;[1 1 1] When active Capture Scene and Update Display
  (if (`/Game/AVRFramework/Blueprints/Components/State/Comp_Active.Active` (`self.Comp_Active`))
    (if (not (`self.GalleryMode`))
      (set `TextureRenderTarget.TargetGamma` 2.0 (`SceneCaptureComponent2D.TextureTarget` (`self.SceneCaptureComponent2DLowres`)))
      (`SceneCaptureComponent2D.CaptureScene` (`self.SceneCaptureComponent2DLowres`)))))

(event `self.Comp_Grab.ActorPickedUp`
  (params (GrabbingPawn :type "/Game/AVRFramework/Blueprints/Pawn/BP_Pawn_Base Object Reference") (GrabbingActor :type "Actor Object Reference") (GrabbingMotionController :type "/Game/AVRFramework/Blueprints/VR/MotionControllers/BP_MotionController Object Reference") (GrabbingMComp :type "/Game/AVRFramework/Blueprints/VR/MotionComponents/BP_MComp Object Reference"))
  ;[1 1 1] Handle Grab - Activates on Grab
  (`/Game/AVRFramework/Blueprints/Components/State/Comp_Active.SetActiv` (`self.Comp_Active`) true))

(event `SetGalleryMode`
  (params (GalleryMode :type Boolean))
  ;[1 1 1] GalleryMode
  (bind _output_get (set `self.GalleryMode` GalleryMode))
  (`SceneComponent.SetVisibility` (`self.Comp_Widget`) _output_get false)
  (`PrimitiveComponent.SetMaterial` (`self.Camera`) 5 (select `bool` _output_get :`false` "/Game/AVRFramework/Blueprints/Devices/Camera/Mat_Camera.Mat_Camera" :`true` "/Game/AVRFramework/Meshes/Devices/Tablet/Mat_Device_Tablet_Plastic_Black.Mat_Device_Tablet_Plastic_Black" :!type "MaterialInterface Object Reference")))

(event `self.Comp_Grab.ActorReleased`
  (params (ReleasingPawn :type "/Game/AVRFramework/Blueprints/Pawn/BP_Pawn_Base Object Reference") (ReleasingActor :type "Actor Object Reference") (ReleasingMotionController :type "/Game/AVRFramework/Blueprints/VR/MotionControllers/BP_MotionController Object Reference") (ReleasingMComp :type "/Game/AVRFramework/Blueprints/VR/MotionComponents/BP_MComp Object Reference"))
  ;[1 1 1] Handle Grab - Activates on Grab
  (`/Game/AVRFramework/Blueprints/Components/State/Comp_Active.SetActiv` (`self.Comp_Active`) false))

(event `self.Comp_Grab.KeyInput`
  (params (Key :type "/Game/AVRFramework/Enums/Enum_Controller_Buttons Enum" :default "NewEnumerator1") (Set :type Boolean))
  ;[1 1 1] Take Photo on Trigger Pressed, taking Pictures creates a Photo Actor
  (switch `/Game/AVRFramework/Enums/Enum_Controller_Buttons` Key
    (:`NewEnumerator0`
      (if Set
        (if (not (`self.GalleryMode`))
          (`self.TakePicture`))))
    (:`NewEnumerator3`
      (if Set
        (`self.SetSelfieMode` (not (`self.SelfieMode`)))))
    (:`NewEnumerator4`
      (if Set
        (`self.SetGalleryMode` (not (`self.GalleryMode`)))))))

(event `SetSelfieMode`
  (params (Set :type Boolean))
  (bind _capturehandle (`self.CaptureHandle`))
  (bind _capturehandle_2 (`self.CaptureHandle`))
  ;[1 1 1] Take Photo on Trigger Pressed, taking Pictures creates a Photo Actor
  (set `self.SelfieMode` Set)
  (bind _out (`/Game/AVRFramework/Libraries/FLib_Utility.SaveVector` (`SceneComponent.RelativeLocation` _capturehandle)))
  (bind _out_2 (`/Game/AVRFramework/Libraries/FLib_Utility.SaveRotator` (`SceneComponent.RelativeRotation` _capturehandle)))
  (bind (_direction _percent) (`Timeline|MoveToLocation` :!via `PlayFromStart`)
    (:`Update`
      (`SceneComponent.K2_SetRelativeLocation` _capturehandle_2 (`KismetMathLibrary.VLerp` _out (select `bool` Set :`false` (0.0 0.0 -3.0) :`true` (0.0 0.0 3.0) :!type "Vector Structure") _percent) false false)
      (`SceneComponent.K2_SetRelativeRotation` _capturehandle_2 (`KismetMathLibrary.RLerp` _out_2 (select `bool` Set :`false` (struct :`Pitch` -90.0 :`Roll` 180.009995) :`true` (struct :`Pitch` 90.0) :!type "Rotator Structure") _percent true) false false))))

(event `TakePicture`
  (bind _scenecapturecomponent2dhighres (`self.SceneCaptureComponent2DHighres`))
  ;[1 1 1] Take Photo on Trigger Pressed, taking Pictures creates a Photo Actor
  (bind _returnvalue (`|SpawnActorFromClass` "/Game/AVRFramework/Blueprints/Helpers/BP_Helper_Photo.BP_Helper_Photo_C" (`KismetMathLibrary.MakeTransform` (0.0 0.0 10000.0)) "AlwaysSpawn" "OverrideRootScale" null "Photo" "This is a Photo" null))
  (bind _texturetarget (`/Game/AVRFramework/Blueprints/Helpers/BP_Helper_Photo.PrintPicture` _returnvalue))
  (set `TextureRenderTarget.TargetGamma` 2.5 _texturetarget)
  (set `SceneCaptureComponent2D.TextureTarget` _texturetarget _scenecapturecomponent2dhighres)
  (`SceneCaptureComponent2D.CaptureScene` _scenecapturecomponent2dhighres)
  (`GameplayStatics.PlaySoundAtLocation` "/Game/AVRFramework/Sound/Cues/Device/Camera/Cue_Device_Camera.Cue_Device_Camera" (`self.K2_GetActorLocation`) (struct) 1.0 1.0 0.0 null null null)
  (`self.PictureTaken`)
  (`/Game/AVRFramework/Libraries/Lib_Core.SetHaptics` (`/Game/AVRFramework/Blueprints/Components/Interaction/Comp_Grab.GrabbingMotionController` (`self.Comp_Grab`)) "NewEnumerator1" "NewEnumerator2" 0.1 1.0))

(event `self.Comp_Widget.WidgetFunctionality`
  (params (Command :type Name) (ReferenceObject :type "Object Object Reference") (ReferenceClass :type "Object Class Reference"))
  ;[1 1 1] Spawn Photo
  (switch `name` Command
    (:`SpawnPhoto`
      (add `/Game/AVRFramework/Blueprints/Components/Util/Comp_Spawner.NewActorSpawned` (`self.Comp_Spawner`) (delegate `NewActorSpawned_Event_0`))
      (`/Game/AVRFramework/Blueprints/Components/Util/Comp_Spawner.SpawnNewActor` (`self.Comp_Spawner`) "/Game/AVRFramework/Blueprints/Devices/Camera/BP_Photo.BP_Photo_C"))))

(event `NewActorSpawned_Event_0`
  (params (SpawnedActor :type "Actor Object Reference"))
  ;[1 1 1] Spawn Photo
  (remove `/Game/AVRFramework/Blueprints/Components/Util/Comp_Spawner.NewActorSpawned` (`self.Comp_Spawner`) (delegate `NewActorSpawned_Event_0`))
  (bind _asbp_photo (cast `/Game/AVRFramework/Blueprints/Devices/Camera/BP_Photo` SpawnedActor))
  (bind _asbp_helper_photo (cast `/Game/AVRFramework/Blueprints/Helpers/BP_Helper_Photo` (stale `self.Comp_Widget.WidgetFunctionality` ReferenceObject)))
  (`/Game/AVRFramework/Blueprints/Devices/Camera/BP_Photo.MakePhoto` _asbp_photo _asbp_helper_photo))

(fn `UserConstructionScript`
  (`parent.UserConstructionScript`))