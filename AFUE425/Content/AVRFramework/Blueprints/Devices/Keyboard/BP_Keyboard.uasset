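; BP_Keyboard is an AVRFramework keyboard device that passes key presses from its on-screen keyboard widget to other actors.
; On BeginPlay it binds KeyPressed to the Widget_Keyboard_Base hosted in its widget component.
; Each press sends the key, string and functional flag through Interface_KeyboardInput to both the connected actor and ActorToForwardKeysTo, whenever each is valid and implements the interface.
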(event `self.ReceiveBeginPlay`
  ;[1 1 1] Setup Keyboard
  (`parent.ReceiveBeginPlay`)
  (bind _aswidget_keyboard_base (cast `/Game/AVRFramework/Blueprints/Widgets/Devices/Keyboard/Widget_Keyboard_Base` (`WidgetComponent.GetUserWidgetObject` (`self.Comp_Widget`))))
  (add `/Game/AVRFramework/Blueprints/Widgets/Devices/Keyboard/Widget_Keyboard_Base.KeyButtonPressed` _aswidget_keyboard_base (delegate `KeyPressed`)))

(event `KeyPressed`
  (params (Key :type "Key Structure" :default "None") (String :type String) (Functional :type Boolean))
  ;[1 1 1] Forward Keyboard Inputs to Attached Actor
  (`|ExecutionSequence`
    (:`then_0`
      (bind (_connector _actor) (`/Game/AVRFramework/Libraries/FLib_Utility.getActorIAmConnectedTo` self))
      (`/Engine/EditorBlueprintResources/StandardMacros.IsValid` _actor
        (:`Is Valid`
          (if (`KismetSystemLibrary.DoesImplementInterface` _actor "/Game/AVRFramework/Interface/Interface_KeyboardInput.Interface_KeyboardInput_C")
            (message `/Game/AVRFramework/Interface/Interface_KeyboardInput.KeyboardInput` _actor String Key Functional)))))
    (:`then_1`
      (bind _actortoforwardkeysto (`self.ActorToForwardKeysTo`)
        (:`then`
          (if (`KismetSystemLibrary.DoesImplementInterface` _actortoforwardkeysto "/Game/AVRFramework/Interface/Interface_KeyboardInput.Interface_KeyboardInput_C")
            (message `/Game/AVRFramework/Interface/Interface_KeyboardInput.KeyboardInput` _actortoforwardkeysto String Key Functional)))
        (:`else`)))))

(fn `UserConstructionScript`
  (`parent.UserConstructionScript`))