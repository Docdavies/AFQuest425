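; Cap actor for a canvas marker in the AVR framework, tinted to a given color.
; On BeginPlay it creates a dynamic instance of the Edding base color material for the Cap component if none is valid yet.
; It then writes its Color variable to that instance's Color parameter.
; Overlap, Tick and the construction script add no logic of their own.
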(event `self.ReceiveBeginPlay`
  (`parent.ReceiveBeginPlay`)
  (`/Engine/EditorBlueprintResources/StandardMacros.IsValid` (`self.CapMaterialInstant`)
    (:`Is Valid`
      _)
    (:`Is Not Valid`
      (bind _returnvalue (`KismetMaterialLibrary.CreateDynamicMaterialInstance` "/Game/AVRFramework/Meshes/Devices/Canvas/Mat_Tools_Edding_BaseColor.Mat_Tools_Edding_BaseColor"))
      (bind _output_get (set `self.CapMaterialInstant` _returnvalue))
      (`PrimitiveComponent.SetMaterial` (`self.Cap`) 0 _output_get)))
  (`MaterialInstanceDynamic.SetVectorParameterValue` (`self.CapMaterialInstant`) "Color" (`self.Color`)))

(fn `UserConstructionScript`
  (`parent.UserConstructionScript`))