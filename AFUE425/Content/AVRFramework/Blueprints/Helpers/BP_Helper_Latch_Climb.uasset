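; VR climbing latch helper that lets a pawn pull itself along by moving the hand latched to this actor.
; On latch, it caches the motion controller component and its relative location.
; While that reference is valid, Tick applies the inverse of the controller's movement as a swept local offset to the pawn and forces Flying mode.
; Release restores Walking, but this Blueprint does not clear the cached controller.
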(event `self.ReceiveTick`
  (params (DeltaSeconds :type "Float (single-precision)"))
  (bind _controllercomponent (`self.ControllerComponent`))
  (bind _relativelocation (`SceneComponent.RelativeLocation` _controllercomponent))
  ;[1 1 1] Extends Climbing Behaviour
  (`parent.ReceiveTick` DeltaSeconds)
  (`/Engine/EditorBlueprintResources/StandardMacros.IsValid` _controllercomponent
    (:`Is Valid`
      (set `self.Difference` (- (`self.LastRelativeLocation`) _relativelocation))
      (set `self.LastRelativeLocation` _relativelocation)
      (`self.K2_AddActorLocalOffset` (`self.LatchingPawn`) (`self.Difference`) true false)
      (`CharacterMovementComponent.SetMovementMode` (`Character.CharacterMovement` (`self.LatchingPawn`)) "MOVE_Flying" 0))))

(event `self.ActorGotLatched`
  (params (LatchingPawn :type "/Game/AVRFramework/Blueprints/Pawn/BP_Pawn_Base Object Reference") (LatchingActor :type "Actor Object Reference") (LatchingMotionController :type "/Game/AVRFramework/Blueprints/VR/MotionControllers/BP_MotionController Object Reference") (LatchingMComp :type "/Game/AVRFramework/Blueprints/VR/MotionComponents/BP_MComp Object Reference"))
  (bind _controllercomponent (`/Game/AVRFramework/Blueprints/VR/MotionComponents/BP_MComp.ControllerComponent` LatchingMComp))
  (`parent.ActorGotLatched` LatchingPawn LatchingActor LatchingMotionController LatchingMComp)
  (`/Engine/EditorBlueprintResources/StandardMacros.IsValid` LatchingMComp
    (:`Is Valid`
      (`/Engine/EditorBlueprintResources/StandardMacros.IsValid` _controllercomponent
        (:`Is Valid`
          (set `self.ControllerComponent` _controllercomponent)
          (set `self.LastRelativeLocation` (`SceneComponent.RelativeLocation` _controllercomponent)))))))

(event `self.ActorLatchReleased`
  (params (ReleasingPawn :type "/Game/AVRFramework/Blueprints/Pawn/BP_Pawn_Base Object Reference") (ReleasingActor :type "Actor Object Reference") (ReleasingMotionController :type "/Game/AVRFramework/Blueprints/VR/MotionControllers/BP_MotionController Object Reference") (ReleasingMComp :type "/Game/AVRFramework/Blueprints/VR/MotionComponents/BP_MComp Object Reference"))
  (`CharacterMovementComponent.SetMovementMode` (`Character.CharacterMovement` (`self.LatchingPawn`)) "MOVE_Walking" 0)
  (`parent.ActorLatchReleased` ReleasingPawn ReleasingActor ReleasingMotionController ReleasingMComp))

(fn `UserConstructionScript`
  (`parent.UserConstructionScript`))