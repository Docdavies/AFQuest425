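; BP_Helper_MeasurementMarker is a VR helper actor that acts as a marker linked to measurement connections.
; Before its delete component removes it, it deletes every actor in MeasurementConnections, passing an animation override with preferred animations disallowed.
; IsInMotion reports true while the marker is not yet placed, or while its grab component has a valid grabbing actor.
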(event `self.ReceiveTick`
  (params (DeltaSeconds :type "Float (single-precision)")))

(event `self.Comp_Delete.BeforeDelete`
  (bind _result (`BlueprintSetLibrary.Set_ToArray` (`self.MeasurementConnections`)))
  (for _array_element _result
    (`/Game/AVRFramework/Libraries/FLib_Utility.DeleteActor` _array_element)))

(fn `IsInMotion`
  (returns (InMotion :type Boolean))
  (if (`self.Placed`)
    (`/Engine/EditorBlueprintResources/StandardMacros.IsValid` (`/Game/AVRFramework/Blueprints/Components/Interaction/Comp_Grab.GrabbingActor` (`self.Comp_Grab`))
      (:`Is Valid`
        (return true))
      (:`Is Not Valid`
        (return false)))
    (else
      (return true))))

(fn `UserConstructionScript`)