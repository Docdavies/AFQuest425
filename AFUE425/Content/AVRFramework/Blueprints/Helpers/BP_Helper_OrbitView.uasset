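; BP_Helper_OrbitView is an orbit-view helper that rotates and zooms a camera through a SpringArm.
; LookUp and LookRight add relative pitch and yaw to the arm, and Zoom changes its length, starting from InitialDistance.
; Pitch and zoom steps that would leave PitchRange or ZoomRange are ignored rather than clamped to the limit; yaw is unrestricted.
; GetCameraPosition returns the camera's world location and rotation.
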(event `LookUp`
  (params (AxisValue :type "Float (double-precision)"))
  (bind (_pitchrange_min _pitchrange_max) (break `InputRange` (`self.PitchRange`)))
  (bind (_relativerotation_roll _relativerotation_pitch) (`KismetMathLibrary.BreakRotator` (`SceneComponent.RelativeRotation` (`self.SpringArm`))))
  (if (`KismetMathLibrary.InRange_FloatFloat` (+ AxisValue (`KismetMathLibrary.FClamp` _relativerotation_pitch -70.0 80.0)) _pitchrange_min _pitchrange_max false false)
    (`SceneComponent.K2_AddRelativeRotation` (`self.SpringArm`) (`KismetMathLibrary.MakeRotator` 0.0 AxisValue) false false)))

(event `LookRight`
  (params (AxisValue :type "Float (double-precision)"))
  (`SceneComponent.K2_AddRelativeRotation` (`self.SpringArm`) (`KismetMathLibrary.MakeRotator` 0.0 0.0 AxisValue) false false))

(event `Zoom`
  (params (Factor :type "Float (double-precision)"))
  (bind (_zoomrange_min _zoomrange_max) (break `InputRange` (`self.ZoomRange`)))
  (bind _returnvalue (+ Factor (`SpringArmComponent.TargetArmLength` (`self.SpringArm`))))
  (if (`KismetMathLibrary.InRange_FloatFloat` _returnvalue _zoomrange_min _zoomrange_max false false)
    (set `SpringArmComponent.TargetArmLength` _returnvalue (`self.SpringArm`))))

(fn `getCameraPosition`
  (returns (Location :type "Vector Structure") (Rotation :type "Rotator Structure"))
  (bind _camera (`self.Camera`))
  (return (`SceneComponent.K2_GetComponentLocation` _camera) (`SceneComponent.K2_GetComponentRotation` _camera)))

(fn `UserConstructionScript`
  (set `SpringArmComponent.TargetArmLength` (`self.InitialDistance`) (`self.SpringArm`)))