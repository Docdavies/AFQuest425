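; BP_Helper_Anchor is a helper actor in the AVRFramework that carries a sphere component with an adjustable, network-aware radius.
; The construction script sets replication from the ShouldReplicate flag, and BeginPlay applies the stored radius to the sphere.
; NewSphereRadius stores and applies a new value, while a RepNotify on SphereRadius reapplies it when replicated, updating overlaps each time.
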(event `self.ReceiveTick`
  (params (DeltaSeconds :type "Float (single-precision)")))

(event `self.ReceiveBeginPlay`
  (`self.SetSphereRadius` (`self.SphereRadius`)))

(event `NewSphereRadius`
  (params (SphereRadius :type "Float (double-precision)"))
  (bind _output_get (set `self.SphereRadius` SphereRadius))
  (`self.SetSphereRadius` _output_get))

(event `SetSphereRadius`
  (params (SphereRadius :type "Float (double-precision)"))
  (`SphereComponent.SetSphereRadius` (`self.Sphere`) SphereRadius true))

(fn `OnRep_SphereRadius`
  (`self.SetSphereRadius` (`self.SphereRadius`)))

(fn `UserConstructionScript`
  (`self.SetReplicates` (`self.ShouldReplicate`)))