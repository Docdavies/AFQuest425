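; BP_Helper_Latch is a VR framework helper Blueprint that tracks what is currently latched onto it.
; On BeginPlay it binds to the latched and released events of its LatchComponent, if that component is valid.
; A latch stores the latching pawn, actor, motion controller and MComp through SetLatchingVariables.
; A release calls the same function with no arguments, clearing those references.
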(event `self.ReceiveTick`
  (params (DeltaSeconds :type "Float (single-precision)")))

(event `self.ReceiveBeginPlay`
  (bind _latchcomponent (`self.LatchComponent`))
  (`/Engine/EditorBlueprintResources/StandardMacros.IsValid` _latchcomponent
    (:`Is Valid`
      (add `/Game/AVRFramework/Blueprints/Components/Interaction/Comp_Latch.ActorGotLatched` _latchcomponent (delegate `ActorGotLatched`))
      (add `/Game/AVRFramework/Blueprints/Components/Interaction/Comp_Latch.ActorLatchReleased` _latchcomponent (delegate `ActorLatchReleased`)))))

(event `ActorGotLatched`
  (params (LatchingPawn :type "/Game/AVRFramework/Blueprints/Pawn/BP_Pawn_Base Object Reference") (LatchingActor :type "Actor Object Reference") (LatchingMotionController :type "/Game/AVRFramework/Blueprints/VR/MotionControllers/BP_MotionController Object Reference") (LatchingMComp :type "/Game/AVRFramework/Blueprints/VR/MotionComponents/BP_MComp Object Reference"))
  (`self.SetLatchingVariables` LatchingPawn LatchingActor LatchingMotionController LatchingMComp))

(event `ActorLatchReleased`
  (params (ReleasingPawn :type "/Game/AVRFramework/Blueprints/Pawn/BP_Pawn_Base Object Reference") (ReleasingActor :type "Actor Object Reference") (ReleasingMotionController :type "/Game/AVRFramework/Blueprints/VR/MotionControllers/BP_MotionController Object Reference") (ReleasingMComp :type "/Game/AVRFramework/Blueprints/VR/MotionComponents/BP_MComp Object Reference"))
  (`self.SetLatchingVariables` null))

(fn `SetLatchingVariables`
  (params (LatchingPawn :type "/Game/AVRFramework/Blueprints/Pawn/BP_Pawn_Base Object Reference") (LatchingActor :type "Actor Object Reference") (LatchingMotionController :type "/Game/AVRFramework/Blueprints/VR/MotionControllers/BP_MotionController Object Reference") (LatchingMComp :type "/Game/AVRFramework/Blueprints/VR/MotionComponents/BP_MComp Object Reference"))
  (set `self.LatchingPawn` LatchingPawn)
  (set `self.LatchingMotionController` LatchingMotionController)
  (set `self.LatchingMComp` LatchingMComp)
  (set `self.LatchingActor` LatchingActor))

(fn `UserConstructionScript`)