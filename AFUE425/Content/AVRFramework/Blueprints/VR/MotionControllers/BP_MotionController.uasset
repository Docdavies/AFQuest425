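; BP_MotionController is the per-hand VR controller actor that registers with the VR pawn and attaches to its motion controller component.
; It maps child-actor MComp modules and routes key input to them as pawn-configured functions, letting a prioritised MComp take over controls.
; It also forwards button highlights and trim color to the controller MComp.
; Locally controlled haptics use timeline curves stretched to the requested duration, scaled by strength and preset multiplier.
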(event `self.ReceiveTick`
  (params (DeltaSeconds :type "Float (single-precision)")))

(event `self.ReceiveBeginPlay`
  (bind _vrpawn (`self.VRPawn`))
  (bind _motioncontrollercomponent (`self.MotionControllerComponent`))
  ;[1 1 1] Setup
  (`parent.ReceiveBeginPlay`)
  (`/Game/AVRFramework/Libraries/MLib_Actor_Macros.WaitForObjectToValidate` _vrpawn
    (:`Is Valid`
      (`/Game/AVRFramework/Blueprints/Pawn/BP_Pawn_Base.RegisterActorToPawn` _vrpawn self true)
      (`BlueprintMapLibrary.Map_Add` (`/Game/AVRFramework/Blueprints/Pawn/BP_Pawn_VR.Controllers` _vrpawn) (`self.Side`) self)
      (`/Game/AVRFramework/Libraries/MLib_Actor_Macros.WaitForObjectToValidate` _motioncontrollercomponent
        (:`Is Valid`
          (`self.K2_AttachToComponent` _motioncontrollercomponent "None" "KeepRelative" "KeepRelative" "KeepRelative" false)
          (`self.UpdateMCompMap`))))))

(event `KeyInput`
  (params (Set :type Boolean) (Key :type "/Game/AVRFramework/Enums/Enum_Controller_Buttons Enum" :default "NewEnumerator1"))
  (bind _prioritisedmcomp (`self.PrioritisedMComp`))
  (bind _function (`/Game/AVRFramework/Blueprints/Components/Info/Comp_Controls.getFunctionFromButtonAndSide` (`/Game/AVRFramework/Blueprints/Pawn/BP_Pawn_VR.Comp_Controller_VR` (`self.VRPawn`)) Key (`self.Side`)))
  ;[1 1 1] Assign Button Actions
  (bind _asbp_mcomp_controller (`self.GetControllerMComp`)
    (:`then`
      (`/Game/AVRFramework/Blueprints/VR/MotionComponents/BP_MComp_Controller.SetButtonHighlight` _asbp_mcomp_controller Key Set))
    (:`CastFailed`
      _))
  (`/Engine/EditorBlueprintResources/StandardMacros.IsValid` (`self.PrioritisedMComp`)
    (:`Is Valid`
      (`/Game/AVRFramework/Blueprints/VR/MotionComponents/BP_MComp.KeyPressed` (`self.PrioritisedMComp`) Key Set))
    (:`Is Not Valid`
      _))
  (if (`|EnumInequality` _function "NewEnumerator0")
    (bind _keys (`BlueprintMapLibrary.Map_Keys` (`self.MCompMap`)))
    (for _array_element _keys
      (bind (_value _returnvalue) (`BlueprintMapLibrary.Map_Find` (`self.MCompMap`) _array_element))
      (if _returnvalue
        (if (or (`|EnumEquality` _function "NewEnumerator2") (`|EnumEquality` _function "NewEnumerator3"))
          (`/Game/AVRFramework/Blueprints/VR/MotionComponents/BP_MComp.FunctionInput` _value _function Set :!label _label)
          (else
            (`/Engine/EditorBlueprintResources/StandardMacros.IsValid` _prioritisedmcomp
              (:`Is Valid`
                (if (== _prioritisedmcomp _value)
                  (goto _label)))
              (:`Is Not Valid`
                (goto _label)))))))))

(event `SetReplacedControls`
  (params (Set :type Boolean) (PriorityMComp :type "/Game/AVRFramework/Blueprints/VR/MotionComponents/BP_MComp Object Reference"))
  ;[1 1 1] Assign Button Actions
  (if Set
    (set `self.PrioritisedMComp` PriorityMComp)
    (else
      (set `self.PrioritisedMComp` null))))

(event `UpdateMCompMap`
  ;[1 1 1] Create MComp Map
  (`BlueprintMapLibrary.Map_Clear` (`self.MCompMap`))
  (for _array_element (`self.K2_GetComponentsByClass` "/Script/Engine.ChildActorComponent")
    (bind _asbp_mcomp (cast `/Game/AVRFramework/Blueprints/VR/MotionComponents/BP_MComp` (`ChildActorComponent.ChildActor` _array_element)))
    (`BlueprintMapLibrary.Map_Add` (`self.MCompMap`) (`/Game/AVRFramework/Blueprints/VR/MotionComponents/BP_MComp.MComp` _asbp_mcomp) _asbp_mcomp)))

(event `DesiredControllerColor`
  (params (DesiredColor :type "LinearColor Structure"))
  ;[1 1 1] AdjustVisuals
  (bind _asbp_mcomp_controller (`self.GetControllerMComp`)
    (:`then`
      (`/Game/AVRFramework/Blueprints/VR/MotionComponents/BP_MComp_Controller.SetTrimColor` _asbp_mcomp_controller DesiredColor))))

(event `SetHaptics`
  (params (Curve :type "/Game/AVRFramework/Enums/Enum_Haptic_Curves Enum" :default "NewEnumerator4") (Duration :type "Float (double-precision)") (Strength :type "Float (double-precision)"))
  (bind _returnvalue (/ 1.0 Duration))
  ;[1 1 1] Haptics
  (`|ExecutionSequence`
    (:`then_0`
      (`self.LocallyControlled`)
      (if (== Duration 0.0)
        (`self.ExecuteHaptic` 0.01 1.0 Strength :!label _label_2)
        (`KismetSystemLibrary.RetriggerableDelay` 0.1)
        (`self.StopHaptics`)
        (else
          (switch `/Game/AVRFramework/Enums/Enum_Haptic_Curves` Curve
            (:`NewEnumerator4`
              (goto _label_2))
            (:`NewEnumerator0`
              (`TimelineComponent.SetPlayRate` (`self.HapticsTimelineConstant`) _returnvalue)
              (bind (_direction _percent) (`Timeline|HapticsTimelineConstant` :!via `PlayFromStart`)
                (:`Update`
                  (`self.ExecuteHaptic` 0.01 _percent Strength))
                (:`Finished`
                  (`self.StopHaptics` :!label _label_3))))
            (:`NewEnumerator1`
              (`TimelineComponent.SetPlayRate` (`self.HapticsTimelineUpCurve`) _returnvalue)
              (bind (_direction_2 _percent_2) (`Timeline|HapticsTimelineUpCurve` :!via `PlayFromStart`)
                (:`Update`
                  (`self.ExecuteHaptic` 0.01 _percent_2 Strength))
                (:`Finished`
                  (goto _label_3))))
            (:`NewEnumerator2`
              (`TimelineComponent.SetPlayRate` (`self.HapticsTimelineDownCurve`) _returnvalue)
              (bind (_direction_3 _percent_3) (`Timeline|HapticsTimelineDownCurve` :!via `PlayFromStart`)
                (:`Update`
                  (`self.ExecuteHaptic` 0.01 _percent_3 Strength))
                (:`Finished`
                  (goto _label_3))))
            (:`NewEnumerator3`
              (`TimelineComponent.SetPlayRate` (`self.HapticsTimelineNormalCurve`) _returnvalue)
              (bind (_direction_4 _percent_4) (`Timeline|HapticsTimelineNormalCurve` :!via `PlayFromStart`)
                (:`Update`
                  (`self.ExecuteHaptic` 0.01 _percent_4 Strength))
                (:`Finished`
                  (goto _label_3))))))))
    (:`then_1`
      (`KismetSystemLibrary.Delay` Duration)
      (`self.StopHaptics`))))

(event `SetMeshVisibility`
  (params (Set :type Boolean))
  ;[1 1 1] Set Visibility
)

(event `ExecuteHaptic`
  (params (Frequency :type "Float (double-precision)" :default 0.01) (Amplitude :type "Float (double-precision)") (StengthMultiplyer :type "Float (double-precision)"))
  ;[1 1 1] Haptics
  (bind _asbp_player_controller_main (cast `/Game/AVRFramework/Blueprints/Game/BP_PlayerController_Main` (`Pawn.GetController` (`self.VRPawn`))))
  (`PlayerController.SetHapticsByValue` _asbp_player_controller_main Frequency (* Amplitude StengthMultiplyer (`/Game/AVRFramework/DataAsset/Presets/VRControls/PDA_ControllerVR.HapticsMultiplyer` (`/Game/AVRFramework/Blueprints/Components/Info/Comp_Controls.getPresetAsset` (`/Game/AVRFramework/Blueprints/Pawn/BP_Pawn_VR.Comp_Controller_VR` (`self.VRPawn`))))) (select `/Game/AVRFramework/Enums/Enum_Side` (`self.Side`) :`NewEnumerator0` "Left" :`NewEnumerator1` "Right" :!type "EControllerHand Enum")))

(event `StopHaptics`
  ;[1 1 1] Stop Haptics again
  (bind _asbp_player_controller_main (cast `/Game/AVRFramework/Blueprints/Game/BP_PlayerController_Main` (`Pawn.GetController` (`self.VRPawn`))))
  (`PlayerController.StopHapticEffect` _asbp_player_controller_main (select `/Game/AVRFramework/Enums/Enum_Side` (`self.Side`) :`NewEnumerator0` "Left" :`NewEnumerator1` "Right" :!type "EControllerHand Enum")))

(fn `getAllAttachedActors`
  (returns (Actors :type "Set of Actor Object Reference"))
  (locals (Return :type "Set of Actor Object Reference"))
  (bind _return (`local.Return`))
  (bind _values (`BlueprintMapLibrary.Map_Values` (`self.MCompMap`)))
  (for _array_element _values
    (`/Engine/EditorBlueprintResources/StandardMacros.IsValid` _array_element
      (:`Is Valid`
        (bind _actors (`/Game/AVRFramework/Blueprints/VR/MotionComponents/BP_MComp.getAllAttachedActors` _array_element))
        (`BlueprintSetLibrary.Set_Union` _return _actors)
        (`BlueprintSetLibrary.Set_Add` _return _array_element))))
  (return (`local.Return`)))

(fn `getGrabbingActor`
  (returns (GrabbingActor :type "Actor Object Reference"))
  (for _array_element (`self.K2_GetComponentsByClass` "/Script/Engine.ChildActorComponent")
    (bind _childactor (`ChildActorComponent.ChildActor` _array_element))
    (`/Game/AVRFramework/Libraries/MLib_Object_Macros.DoesImplementInterface` _childactor "/Game/AVRFramework/Interface/Interface_GrabbingActor.Interface_GrabbingActor_C"
      (:`true`
        (return _childactor))))
  (return null))

(fn `UserConstructionScript`)