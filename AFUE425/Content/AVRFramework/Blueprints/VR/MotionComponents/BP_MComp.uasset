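; BP_MComp is a base actor for modular motion controller components in the VR framework, spawned as a child of BP_MotionController.
; On BeginPlay it waits for valid references, adds itself to the controller's MCompMap and registers with the VR pawn as its owner.
; It then caches side, pawn and controller references and applies its active state.
; Input, visibility and attached-actor hooks are empty stubs for subclasses.
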(event `self.ReceiveBeginPlay`
  (bind _returnvalue (`self.GetParentActor`))
  (`/Game/AVRFramework/Libraries/MLib_Actor_Macros.WaitForObjectToValidate` _returnvalue
    (:`Is Valid`
      ;[1 1 1] Setup
      (bind _asbp_motion_controller (cast `/Game/AVRFramework/Blueprints/VR/MotionControllers/BP_MotionController` _returnvalue))
      (`BlueprintMapLibrary.Map_Add` (`/Game/AVRFramework/Blueprints/VR/MotionControllers/BP_MotionController.MCompMap` _asbp_motion_controller) (`self.MComp`) self)
      (bind _vrpawn (`/Game/AVRFramework/Blueprints/VR/MotionControllers/BP_MotionController.VRPawn` _asbp_motion_controller))
      (`/Game/AVRFramework/Libraries/MLib_Actor_Macros.WaitForObjectToValidate` _vrpawn
        (:`Is Valid`
          (`/Game/AVRFramework/Blueprints/Pawn/BP_Pawn_Base.RegisterActorToPawn` _vrpawn self true)
          (`self.SetOwner` _vrpawn)
          (bind _motioncontrollercomponent (`/Game/AVRFramework/Blueprints/VR/MotionControllers/BP_MotionController.MotionControllerComponent` _asbp_motion_controller))
          (`/Game/AVRFramework/Libraries/MLib_Actor_Macros.WaitForObjectToValidate` _motioncontrollercomponent
            (:`Is Valid`
              (`self.Setup` (`/Game/AVRFramework/Blueprints/VR/MotionControllers/BP_MotionController.Side` _asbp_motion_controller) _vrpawn _motioncontrollercomponent _asbp_motion_controller)
              (`self.MCompSetActive` (`self.Active`)))))))))

(event `self.ReceiveTick`
  (params (DeltaSeconds :type "Float (single-precision)")))

(event `MCompSetActive`
  (params (Set :type Boolean))
  ;[1 1 1] Active Interface
  (set `self.Active` Set))

(event `MCompToggleActive`
  ;[1 1 1] Active Interface
  (`self.MCompSetActive` (not (`self.Active`))))

(event `KeyPressed`
  (params (Key :type "/Game/AVRFramework/Enums/Enum_Controller_Buttons Enum" :default "NewEnumerator1") (Set :type Boolean))
  ;[1 1 1] Override KeyInput
)

(event `FunctionInput`
  (params (Function :type "/Game/AVRFramework/Enums/Enum_Control_Function Enum" :default "NewEnumerator0") (Set :type Boolean))
  ;[1 1 1] Override Function Input
)

(fn `getAllAttachedActors`
  (returns (Actors :type "Set of Actor Object Reference"))
  (return))

(fn `Setup`
  (params (Side :type "/Game/AVRFramework/Enums/Enum_Side Enum" :default "NewEnumerator0") (VRPawn :type "/Game/AVRFramework/Blueprints/Pawn/BP_Pawn_VR Object Reference") (MotionComponent :type "MotionControllerComponent Object Reference") (MotionContoller :type "/Game/AVRFramework/Blueprints/VR/MotionControllers/BP_MotionController Object Reference"))
  (returns (Success :type Boolean))
  (set `self.Side` Side)
  (set `self.VRPawn` VRPawn)
  (set `self.ControllerComponent` MotionComponent)
  (set `self.BaseMotionController` MotionContoller)
  (return true))

(fn `SetVisibility`
  (params (Set :type Boolean)))

(fn `UserConstructionScript`)